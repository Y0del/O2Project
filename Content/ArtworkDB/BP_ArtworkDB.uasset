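; BP_ArtworkDB is an artwork display actor that shows an image from a Firestore artworks collection on a plane.
; On BeginPlay it fetches the collection via VaRest and uses its first actor tag as the index of the document to show.
; It downloads that artwork's image into a dynamic M_ArtFrame_Dynamic material, then scales the plane to the stored aspect ratio, with Size as the shorter side.
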(event Custom|GetProducts
  (params (Request :type Va%20Rest%20Request%20JSON%20Object%20Reference))
  (Class|VaRestSubsystem|CallURL (|VaRestSubsystem) "https://firestore.googleapis.com/v1/projects/image-22b8e/databases/(default)/documents/artworks?key=AIzaSyCC9siV3BqjM5dc3fJKqnMJyeupD5PW3yU" "GET" "x_www_form_urlencoded_url" 0 (delegate Custom|RespondProducts)))

(event Custom|RespondProducts
  (params (Request :type Va%20Rest%20Request%20JSON%20Object%20Reference))
  (bind _returnvalue (Class|VaRestJsonValue|AsObject (Utilities|Array|Get(acopy) (Class|VaRestJsonObject|GetArrayField (Class|VaRestRequestJSON|GetResponseObject Request) "documents") (Math|Conversions|ToInteger(Byte) (Utilities|String|ToString(Name) (Utilities|Array|Get(acopy) (Variables|Actor|GetTags)))))))
  (bind _texture (|DownloadImage (.image_url_string (|ArtworkInfo (Class|VaRestJsonObject|GetObjectField _returnvalue "fields") (Class|VaRestJsonObject|GetObjectField _returnvalue "fields") (Class|VaRestJsonObject|GetObjectField _returnvalue "fields") (Class|VaRestJsonObject|GetObjectField _returnvalue "fields") (Class|VaRestJsonObject|GetObjectField _returnvalue "fields") (Class|VaRestJsonObject|GetObjectField _returnvalue "fields"))))
    (:OnSuccess
      (Variables|Default|SetWidth (Math|Conversions|ToFloat(Integer) (.width_string (|ArtworkInfo (Class|VaRestJsonObject|GetObjectField _returnvalue "fields") (Class|VaRestJsonObject|GetObjectField _returnvalue "fields") (Class|VaRestJsonObject|GetObjectField _returnvalue "fields") (Class|VaRestJsonObject|GetObjectField _returnvalue "fields") (Class|VaRestJsonObject|GetObjectField _returnvalue "fields") (Class|VaRestJsonObject|GetObjectField _returnvalue "fields")))))
      (Variables|Default|SetHeight (Math|Conversions|ToFloat(Integer) (.height_string (|ArtworkInfo (Class|VaRestJsonObject|GetObjectField _returnvalue "fields") (Class|VaRestJsonObject|GetObjectField _returnvalue "fields") (Class|VaRestJsonObject|GetObjectField _returnvalue "fields") (Class|VaRestJsonObject|GetObjectField _returnvalue "fields") (Class|VaRestJsonObject|GetObjectField _returnvalue "fields") (Class|VaRestJsonObject|GetObjectField _returnvalue "fields")))))
      (bind _returnvalue_2 (Rendering|Material|CreateDynamicMaterialInstance "/Game/ArtworkDB/Materials/M_ArtFrame_Dynamic.M_ArtFrame_Dynamic" "None" "None" :!class /Script/Engine.KismetMaterialLibrary))
      (Rendering|Material|SetMaterial (Variables|Default|GetPlane) 0 _returnvalue_2)
      (Rendering|Material|SetTextureParameterValue _returnvalue_2 "ArtworkTexture" _texture)
      (if (> (Variables|Default|GetWidth) (Variables|Default|GetHeight))
        (|Width/Height)
        (else
          (|Height/Width))))))

(event EventBeginPlay
  (CallFunction|GetProducts))

(fn ConstructionScript)